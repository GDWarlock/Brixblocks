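; Brick actor for a ball-and-brick game that loses hit points when struck and destroys itself when they run out.
; On BeginPlay it creates a BrickNumber widget, passes itself as a reference, and shows it through its NumberComponent widget component.
; A HitbyBall event decrements hit points, destroying the brick at zero or below, and plays an explosion sound.
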(event EventBeginPlay
  (bind _returnvalue (UserInterface|CreateWidget "/Game/HUD/BrickNumber.BrickNumber_C"))
  (Variables|/Game/HUD/BrickNumber.BrickNumber_C|SetRefToBrick _returnvalue self)
  (UserInterface|SetWidget (Variables|Default|GetNumberComponent) _returnvalue))

(event Collision|EventActorBeginOverlap
  (params (OtherActor :type Actor%20Object%20Reference)))

(event EventTick
  (params (DeltaSeconds :type Float%20%28single-precision%29)))

(event EventHitbyBall
  (CallFunction|DecrementHitpoints)
  (Audio|PlaySound2D "/Game/StarterContent/Audio/Explosion02.Explosion02" 1.0 1.0 0.0 0 0))

(fn ConstructionScript)

(fn DecrementHitpoints
  (if (<= (- (Variables|Default|GetHitPoints) 1) 0)
    (Actor|DestroyActor)
    (else
      (Math|Integer|DecrementInt (Variables|Default|GetHitPoints)))))